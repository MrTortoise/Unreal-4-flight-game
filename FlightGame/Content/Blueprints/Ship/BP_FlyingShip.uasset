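; Player-controlled flying ship with custom six-degree-of-freedom Newtonian flight, a HUD widget and debug velocity printouts.
; Axis inputs set thrust and torque percentages, which Tick converts through mass and inertia into local-space velocities, counter-rotating linear velocity to preserve momentum.
; Held assists compute clamped counter-thrust to cancel rotation or sideways drift.
; Swept hits reflect velocity scaled by elasticity; force field overlaps and shield strength are stubs.
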(event OnComponentBeginOverlap(ForceFieldBoundary)
  (params (OtherActor :type Actor%20Object%20Reference) (OtherComp :type Primitive%20Component%20Object%20Reference) (OtherBodyIndex :type Integer) (bFromSweep :type Boolean) (SweepResult :type Hit%20Result%20Structure%20%28by%20ref%29)))

(event OnComponentEndOverlap(ForceFieldBoundary)
  (params (OtherActor :type Actor%20Object%20Reference) (OtherComp :type Primitive%20Component%20Object%20Reference) (OtherBodyIndex :type Integer)))

(event EventTick
  (params (DeltaSeconds :type Float%20%28single-precision%29))
  ;[1 1 1] Calculate linear and rotational accelerations, apply to velocities and update location and rotation
  (bind _linearacceleration (CallFunction|GetLinearAcceleration))
  (Development|PrintString (Utilities|String|BuildString(Vector) "" "Linear Velocity:" (+ (* _linearacceleration DeltaSeconds) (Variables|Default|GetCurrentVelocity))) false false)
  (Variables|Default|SetCurrentVelocity (+ (* _linearacceleration DeltaSeconds) (Variables|Default|GetCurrentVelocity)))
  (Transformation|AddActorLocalOffset (* (Variables|Default|GetCurrentVelocity) (Utilities|Time|GetWorldDeltaSeconds)) true)
  (bind _angularacceleration (CallFunction|GetAngularAcceleration))
  (Variables|Default|SetCurrentAngularVelocity (Math|Rotator|CombineRotators (* _angularacceleration (Utilities|Time|GetWorldDeltaSeconds)) (Variables|Default|GetCurrentAngularVelocity)))
  (Transformation|AddActorLocalRotation (* (Variables|Default|GetCurrentAngularVelocity) (Utilities|Time|GetWorldDeltaSeconds)) false)
  (Variables|Default|SetCurrentVelocity (Math|Vector|RotateVector (Variables|Default|GetCurrentVelocity) (Class|KismetMathLibrary|NegateRotator (* (Variables|Default|GetCurrentAngularVelocity) (Utilities|Time|GetWorldDeltaSeconds))))))

(event EventBeginPlay
  ;[1 1 1] Begin Play - setup the HUD
  (bind _returnvalue (UserInterface|CreateWidget "/Game/Blueprints/Ship/FlyingShip_HUD.FlyingShip_HUD_C"))
  (Variables|Default|SetShipHUDWidget _returnvalue)
  (UserInterface|Viewport|AddtoViewport (Variables|Default|GetShipHUDWidget)))

(event EventHit
  (params (MyComp :type Primitive%20Component%20Object%20Reference) (Other :type Actor%20Object%20Reference) (OtherComp :type Primitive%20Component%20Object%20Reference) (bSelfMoved :type Boolean) (HitLocation :type Vector :default "0, 0, 0") (HitNormal :type Vector :default "0, 0, 0") (NormalImpulse :type Vector :default "0, 0, 0") (Hit :type Hit%20Result%20Structure%20%28by%20ref%29))
  ;[1 1 1] Simple reflaction collision with a scalar for coefficient
  (Variables|Default|SetCurrentVelocity (* (Math|Vector|MirrorVectorbyNormal (Variables|Default|GetCurrentVelocity) (Math|Vector|MakeVector (Math|Vector|DotProduct HitNormal (Transformation|GetActorForwardVector)) (Math|Vector|DotProduct HitNormal (Transformation|GetActorRightVector)) (Math|Vector|DotProduct HitNormal (Transformation|GetActorUpVector)))) (Variables|Default|GetCollisionElasticity))))

(event Input|ActionEvents|InputActionAlignMotionForward
  ;[1 1 1] Brake Strafe / Align motion to forward vector
  (:Pressed
    (Variables|Default|SetIsVelocityForwardAlignmentActive true))
  (:Released
    (Variables|Default|SetIsVelocityForwardAlignmentActive false)))

(event Input|ActionEvents|InputActionBrakeRotation
  ;[1 1 1] Brake Rotation
  (:Pressed
    (Variables|Default|SetIsRotationBrakingActive true))
  (:Released
    (Variables|Default|SetIsRotationBrakingActive false)))

(event Input|AxisEvents|InputAxisThrust
  (params (AxisValue :type Float%20%28single-precision%29))
  ;[1 1 1] Calculate X part of thrust percent
  (Variables|Default|SetCurrentLinearThrustPercent (Math|Vector|MakeVector AxisValue (.Y (Math|Vector|BreakVector (Variables|Default|GetCurrentLinearThrustPercent))) (.Z (Math|Vector|BreakVector (Variables|Default|GetCurrentLinearThrustPercent))))))

(event Input|AxisEvents|InputAxisStrafeHorizontal
  (params (AxisValue :type Float%20%28single-precision%29))
  ;[1 1 1] Calculate horizontal linear thrust (strafe)
  (if (not (Variables|Default|GetIsVelocityForwardAlignmentActive))
    (Variables|Default|SetCurrentLinearThrustPercent (Math|Vector|MakeVector (.X (Math|Vector|BreakVector (Variables|Default|GetCurrentLinearThrustPercent))) AxisValue (.Z (Math|Vector|BreakVector (Variables|Default|GetCurrentLinearThrustPercent)))))))

(event Input|AxisEvents|InputAxisStrafeVertical
  (params (AxisValue :type Float%20%28single-precision%29))
  ;[1 1 1] Calculate Vertical Linear Thrust (strafe)
  (if (not (Variables|Default|GetIsVelocityForwardAlignmentActive))
    (Variables|Default|SetCurrentLinearThrustPercent (Math|Vector|MakeVector (.X (Math|Vector|BreakVector (Variables|Default|GetCurrentLinearThrustPercent))) (.Y (Math|Vector|BreakVector (Variables|Default|GetCurrentLinearThrustPercent))) AxisValue))))

(event Input|AxisEvents|InputAxisPitch
  (params (AxisValue :type Float%20%28single-precision%29))
  ;[1 1 1] Calculate pitch Torque Percent
  (if (not (Variables|Default|GetIsRotationBrakingActive))
    (Variables|Default|SetCurrentTorquePercent (Math|Vector|MakeVector AxisValue (.Y (Math|Vector|BreakVector (Variables|Default|GetCurrentTorquePercent))) (.Z (Math|Vector|BreakVector (Variables|Default|GetCurrentTorquePercent)))))))

(event Input|AxisEvents|InputAxisYaw
  (params (AxisValue :type Float%20%28single-precision%29))
  ;[1 1 1] Calculate Yaw Torque Percent
  (if (not (Variables|Default|GetIsRotationBrakingActive))
    (Variables|Default|SetCurrentTorquePercent (Math|Vector|MakeVector (.X (Math|Vector|BreakVector (Variables|Default|GetCurrentTorquePercent))) AxisValue (.Z (Math|Vector|BreakVector (Variables|Default|GetCurrentTorquePercent)))))))

(event Input|AxisEvents|InputAxisRoll
  (params (AxisValue :type Float%20%28single-precision%29))
  ;[1 1 1] Calculate Yaw Roll Percent
  (if (not (Variables|Default|GetIsRotationBrakingActive))
    (Variables|Default|SetCurrentTorquePercent (Math|Vector|MakeVector (.X (Math|Vector|BreakVector (Variables|Default|GetCurrentTorquePercent))) (.Y (Math|Vector|BreakVector (Variables|Default|GetCurrentTorquePercent))) AxisValue))))

(fn ConstructionScript)

(fn GetLinearAcceleration
  (bind _maxstrafethrust (Variables|Default|GetMaxStrafeThrust))
  (if (Variables|Default|GetIsVelocityForwardAlignmentActive)
    (bind _outputlinearthrustpercent (CallFunction|GetStrafeThrusttoBreak))
    (LocalVariables|SetLinearThrustPercent _outputlinearthrustpercent)
    (else
      (LocalVariables|SetLinearThrustPercent (Variables|Default|GetCurrentLinearThrustPercent))))
  (if (< (.X (Math|Vector|BreakVector (LocalVariables|GetLinearThrustPercent))) 0.0)
    (LocalVariables|SetLinearThrust (Math|Vector|MakeVector (* (.X (Math|Vector|BreakVector (LocalVariables|GetLinearThrustPercent))) (Math|Conversions|ToFloat(Integer) (Variables|Default|GetMaxReverseThrust)) -1.0) (* _maxstrafethrust (.Y (Math|Vector|BreakVector (LocalVariables|GetLinearThrustPercent)))) (* _maxstrafethrust (.Z (Math|Vector|BreakVector (LocalVariables|GetLinearThrustPercent))))))
    (else
      (LocalVariables|SetLinearThrust (Math|Vector|MakeVector (* (Math|Conversions|ToFloat(Integer) (Variables|Default|GetMaxForwardThrust)) (.X (Math|Vector|BreakVector (LocalVariables|GetLinearThrustPercent)))) (* _maxstrafethrust (.Y (Math|Vector|BreakVector (LocalVariables|GetLinearThrustPercent)))) (* _maxstrafethrust (.Z (Math|Vector|BreakVector (LocalVariables|GetLinearThrustPercent))))))))
  (return (/ (LocalVariables|GetLinearThrust) (Math|Conversions|ToFloat(Integer) (Variables|Default|GetMass)))))

(fn GetAngularAcceleration
  (bind _momentofinertia (Variables|Default|GetMomentOfInertia))
  (bind _currentangularvelocity (Variables|Default|GetCurrentAngularVelocity))
  (bind _momentofinertia_2 (Variables|Default|GetMomentOfInertia))
  (bind (_x _y _z) (Math|Vector|BreakVector _momentofinertia))
  (bind (_pitch _yaw _roll) (Class|KismetMathLibrary|BreakRot _currentangularvelocity))
  (bind (_x_2 _y_2 _z_2) (Math|Vector|BreakVector _momentofinertia_2))
  (if (Variables|Default|GetIsRotationBrakingActive)
    (bind _angularthrustpercent (CallFunction|GetAngularThrustPercenttoBrake _pitch _x_2))
    (bind _angularthrustpercent_2 (CallFunction|GetAngularThrustPercenttoBrake _yaw _y_2))
    (bind _angularthrustpercent_3 (CallFunction|GetAngularThrustPercenttoBrake _roll _z_2))
    (LocalVariables|SetadjustedTorquePercent (Math|Vector|MakeVector _angularthrustpercent _angularthrustpercent_2 _angularthrustpercent_3))
    (else
      (LocalVariables|SetadjustedTorquePercent (Variables|Default|GetCurrentTorquePercent))))
  (Development|PrintString (Class|KismetStringLibrary|BuildStringRotator "" "Angular Acceleration:" (Class|KismetMathLibrary|MakeRot (/ (.X (Math|Vector|BreakVector (* (LocalVariables|GetadjustedTorquePercent) (Math|Conversions|ToFloat(Integer) (Variables|Default|GetMaxTorque))))) _x) (/ (.Y (Math|Vector|BreakVector (* (LocalVariables|GetadjustedTorquePercent) (Math|Conversions|ToFloat(Integer) (Variables|Default|GetMaxTorque))))) _y) (/ (.Z (Math|Vector|BreakVector (* (LocalVariables|GetadjustedTorquePercent) (Math|Conversions|ToFloat(Integer) (Variables|Default|GetMaxTorque))))) _z))) true false)
  (return (Class|KismetMathLibrary|MakeRot (/ (.X (Math|Vector|BreakVector (* (LocalVariables|GetadjustedTorquePercent) (Math|Conversions|ToFloat(Integer) (Variables|Default|GetMaxTorque))))) _x) (/ (.Y (Math|Vector|BreakVector (* (LocalVariables|GetadjustedTorquePercent) (Math|Conversions|ToFloat(Integer) (Variables|Default|GetMaxTorque))))) _y) (/ (.Z (Math|Vector|BreakVector (* (LocalVariables|GetadjustedTorquePercent) (Math|Conversions|ToFloat(Integer) (Variables|Default|GetMaxTorque))))) _z))))

(fn GetAngularThrustPercenttoBrake
  (params (CurrentAngularVelocity :type Float%20%28single-precision%29) (MomentOfInertia :type Float%20%28single-precision%29))
  (if (!= CurrentAngularVelocity 0.0)
    (LocalVariables|SetATP (* (Math|Float|Clamp(Float) (/ (* MomentOfInertia (/ CurrentAngularVelocity (Utilities|Time|GetWorldDeltaSeconds))) (Math|Conversions|ToFloat(Integer) (Variables|Default|GetMaxTorque))) -1.0 1.0) -1.0))
    (else
      (LocalVariables|SetATP 0.0)))
  (return (LocalVariables|GetATP)))

(fn GetStrafeThrusttoBreak
  (bind _currentvelocity (Variables|Default|GetCurrentVelocity))
  (bind _currentvelocity_2 (Variables|Default|GetCurrentVelocity))
  (bind _z (Math|Vector|BreakVector _currentvelocity))
  (bind _y (Math|Vector|BreakVector _currentvelocity_2))
  (if (!= _y 0.0)
    (LocalVariables|SetthrustPercentY (Math|Float|Clamp(Float) (- 0.0 (/ (* (Variables|Default|GetMass) (/ _y (Utilities|Time|GetWorldDeltaSeconds))) (Math|Conversions|ToFloat(Integer) (Variables|Default|GetMaxStrafeThrust)))) -1.0))
    (else
      (LocalVariables|SetthrustPercentY 0.0)))
  (if (!= _z 0.0)
    (LocalVariables|SetthrustPercentZ (Math|Float|Clamp(Float) (- 0.0 (/ (* (Variables|Default|GetMass) (/ _z (Utilities|Time|GetWorldDeltaSeconds))) (Math|Conversions|ToFloat(Integer) (Variables|Default|GetMaxStrafeThrust)))) -1.0))
    (else
      (LocalVariables|SetthrustPercentZ 0.0)))
  (return (Math|Vector|MakeVector (.X (Math|Vector|BreakVector (Variables|Default|GetCurrentLinearThrustPercent))) (LocalVariables|GetthrustPercentY) (LocalVariables|GetthrustPercentZ))))

(fn GetShieldStrength
  (return 0.0))