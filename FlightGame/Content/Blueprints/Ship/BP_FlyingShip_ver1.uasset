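; Player-flown ship with six-degree-of-freedom inertial flight that also creates its HUD on BeginPlay.
; Input axes set thrust and torque percentages, which become accelerations via mass and moment of inertia and are integrated manually each Tick.
; Local-space velocity is counter-rotated after each turn to preserve world momentum.
; Held brake inputs override player control with computed, limit-capped torque for rotation or strafe thrust to cancel sideways and vertical drift.
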(event EventTick
  (params (DeltaSeconds :type Float%20%28single-precision%29))
  ;[1 1 1] Calculate linear and rotational accelerations, apply to velocities and update location and rotation
  (bind _linearacceleration (CallFunction|GetLinearAcceleration))
  (Development|PrintString (Utilities|String|BuildString(Vector) "" "Linear Velocity:" (+ (* _linearacceleration DeltaSeconds) (Variables|Default|GetCurrentVelocity))) false false)
  (Variables|Default|SetCurrentVelocity (+ (* _linearacceleration DeltaSeconds) (Variables|Default|GetCurrentVelocity)))
  (Transformation|AddActorLocalOffset (* (Variables|Default|GetCurrentVelocity) (Utilities|Time|GetWorldDeltaSeconds)) true)
  (bind _angularacceleration (CallFunction|GetAngularAcceleration))
  (Variables|Default|SetCurrentAngularVelocity (Math|Rotator|CombineRotators (* _angularacceleration (Utilities|Time|GetWorldDeltaSeconds)) (Variables|Default|GetCurrentAngularVelocity)))
  (Transformation|AddActorLocalRotation (* (Variables|Default|GetCurrentAngularVelocity) (Utilities|Time|GetWorldDeltaSeconds)) false)
  (Variables|Default|SetCurrentVelocity (Math|Vector|RotateVector (Variables|Default|GetCurrentVelocity) (Class|KismetMathLibrary|NegateRotator (* (Variables|Default|GetCurrentAngularVelocity) (Utilities|Time|GetWorldDeltaSeconds))))))

(event EventBeginPlay
  ;[1 1 1] Begin Play - setup the HUD
  (bind _returnvalue (UserInterface|CreateWidget "/Game/Blueprints/Ship/FlyingShip_HUD.FlyingShip_HUD_C"))
  (Variables|Default|SetShipHUDWidget _returnvalue)
  (UserInterface|Viewport|AddtoViewport (Variables|Default|GetShipHUDWidget)))

(event Input|ActionEvents|InputActionAlignMotionForward
  ;[1 1 1] Brake Strafe / Align motion to forward vector
  (:Pressed
    (Variables|Default|SetIsVelocityForwardAlignmentActive true))
  (:Released
    (Variables|Default|SetIsVelocityForwardAlignmentActive false)))

(event Input|ActionEvents|InputActionBrakeRotation
  ;[1 1 1] Brake Rotation
  (:Pressed
    (Variables|Default|SetIsRotationBrakingActive true))
  (:Released
    (Variables|Default|SetIsRotationBrakingActive false)))

(event Input|AxisEvents|InputAxisThrust
  (params (AxisValue :type Float%20%28single-precision%29))
  ;[1 1 1] Calculate X part of thrust percent
  (Variables|Default|SetCurrentLinearThrustPercent (Math|Vector|MakeVector AxisValue (.Y (Math|Vector|BreakVector (Variables|Default|GetCurrentLinearThrustPercent))) (.Z (Math|Vector|BreakVector (Variables|Default|GetCurrentLinearThrustPercent))))))

(event Input|AxisEvents|InputAxisStrafeHorizontal
  (params (AxisValue :type Float%20%28single-precision%29))
  ;[1 1 1] Calculate horizontal linear thrust (strafe)
  (if (not (Variables|Default|GetIsVelocityForwardAlignmentActive))
    (Variables|Default|SetCurrentLinearThrustPercent (Math|Vector|MakeVector (.X (Math|Vector|BreakVector (Variables|Default|GetCurrentLinearThrustPercent))) AxisValue (.Z (Math|Vector|BreakVector (Variables|Default|GetCurrentLinearThrustPercent)))))))

(event Input|AxisEvents|InputAxisStrafeVertical
  (params (AxisValue :type Float%20%28single-precision%29))
  ;[1 1 1] Calculate Vertical Linear Thrust (strafe)
  (if (not (Variables|Default|GetIsVelocityForwardAlignmentActive))
    (Variables|Default|SetCurrentLinearThrustPercent (Math|Vector|MakeVector (.X (Math|Vector|BreakVector (Variables|Default|GetCurrentLinearThrustPercent))) (.Y (Math|Vector|BreakVector (Variables|Default|GetCurrentLinearThrustPercent))) AxisValue))))

(event Input|AxisEvents|InputAxisPitch
  (params (AxisValue :type Float%20%28single-precision%29))
  ;[1 1 1] Calculate pitch Torque Percent
  (if (not (Variables|Default|GetIsRotationBrakingActive))
    (Variables|Default|SetCurrentTorquePercent (Math|Vector|MakeVector AxisValue (.Y (Math|Vector|BreakVector (Variables|Default|GetCurrentTorquePercent))) (.Z (Math|Vector|BreakVector (Variables|Default|GetCurrentTorquePercent)))))))

(event Input|AxisEvents|InputAxisYaw
  (params (AxisValue :type Float%20%28single-precision%29))
  ;[1 1 1] Calculate Yaw Torque Percent
  (if (not (Variables|Default|GetIsRotationBrakingActive))
    (Variables|Default|SetCurrentTorquePercent (Math|Vector|MakeVector (.X (Math|Vector|BreakVector (Variables|Default|GetCurrentTorquePercent))) AxisValue (.Z (Math|Vector|BreakVector (Variables|Default|GetCurrentTorquePercent)))))))

(event Input|AxisEvents|InputAxisRoll
  (params (AxisValue :type Float%20%28single-precision%29))
  ;[1 1 1] Calculate Yaw Roll Percent
  (if (not (Variables|Default|GetIsRotationBrakingActive))
    (Variables|Default|SetCurrentTorquePercent (Math|Vector|MakeVector (.X (Math|Vector|BreakVector (Variables|Default|GetCurrentTorquePercent))) (.Y (Math|Vector|BreakVector (Variables|Default|GetCurrentTorquePercent))) AxisValue))))

(fn ConstructionScript)

(fn GetLinearAcceleration
  (bind _maxstrafethrust (Variables|Default|GetMaxStrafeThrust))
  (if (Variables|Default|GetIsVelocityForwardAlignmentActive)
    (bind _outputlinearthrustpercent (CallFunction|GetStrafeThrusttoBreak))
    (LocalVariables|SetLinearThrustPercent _outputlinearthrustpercent)
    (else
      (LocalVariables|SetLinearThrustPercent (Variables|Default|GetCurrentLinearThrustPercent))))
  (if (< (.X (Math|Vector|BreakVector (LocalVariables|GetLinearThrustPercent))) 0.0)
    (LocalVariables|SetLinearThrust (Math|Vector|MakeVector (* (.X (Math|Vector|BreakVector (LocalVariables|GetLinearThrustPercent))) (Math|Conversions|ToFloat(Integer) (Variables|Default|GetMaxReverseThrust)) -1.0) (* _maxstrafethrust (.Y (Math|Vector|BreakVector (LocalVariables|GetLinearThrustPercent)))) (* _maxstrafethrust (.Z (Math|Vector|BreakVector (LocalVariables|GetLinearThrustPercent))))))
    (else
      (LocalVariables|SetLinearThrust (Math|Vector|MakeVector (* (Math|Conversions|ToFloat(Integer) (Variables|Default|GetMaxForwardThrust)) (.X (Math|Vector|BreakVector (LocalVariables|GetLinearThrustPercent)))) (* _maxstrafethrust (.Y (Math|Vector|BreakVector (LocalVariables|GetLinearThrustPercent)))) (* _maxstrafethrust (.Z (Math|Vector|BreakVector (LocalVariables|GetLinearThrustPercent))))))))
  (return (/ (LocalVariables|GetLinearThrust) (Math|Conversions|ToFloat(Integer) (Variables|Default|GetMass)))))

(fn GetAngularAcceleration
  (bind _momentofinertia (Variables|Default|GetMomentOfInertia))
  (bind _currentangularvelocity (Variables|Default|GetCurrentAngularVelocity))
  (bind _momentofinertia_2 (Variables|Default|GetMomentOfInertia))
  (bind (_x _y _z) (Math|Vector|BreakVector _momentofinertia))
  (bind (_pitch _yaw _roll) (Class|KismetMathLibrary|BreakRot _currentangularvelocity))
  (bind (_x_2 _y_2 _z_2) (Math|Vector|BreakVector _momentofinertia_2))
  (if (Variables|Default|GetIsRotationBrakingActive)
    (bind _angularthrustpercent (CallFunction|GetAngularThrustPercenttoBrake _pitch _x_2))
    (bind _angularthrustpercent_2 (CallFunction|GetAngularThrustPercenttoBrake _yaw _y_2))
    (bind _angularthrustpercent_3 (CallFunction|GetAngularThrustPercenttoBrake _roll _z_2))
    (LocalVariables|SetadjustedTorquePercent (Math|Vector|MakeVector _angularthrustpercent _angularthrustpercent_2 _angularthrustpercent_3))
    (else
      (LocalVariables|SetadjustedTorquePercent (Variables|Default|GetCurrentTorquePercent))))
  (Development|PrintString (Class|KismetStringLibrary|BuildStringRotator "" "Angular Acceleration:" (Class|KismetMathLibrary|MakeRot (/ (.X (Math|Vector|BreakVector (* (LocalVariables|GetadjustedTorquePercent) (Math|Conversions|ToFloat(Integer) (Variables|Default|GetMaxTorque))))) _x) (/ (.Y (Math|Vector|BreakVector (* (LocalVariables|GetadjustedTorquePercent) (Math|Conversions|ToFloat(Integer) (Variables|Default|GetMaxTorque))))) _y) (/ (.Z (Math|Vector|BreakVector (* (LocalVariables|GetadjustedTorquePercent) (Math|Conversions|ToFloat(Integer) (Variables|Default|GetMaxTorque))))) _z))) true false)
  (return (Class|KismetMathLibrary|MakeRot (/ (.X (Math|Vector|BreakVector (* (LocalVariables|GetadjustedTorquePercent) (Math|Conversions|ToFloat(Integer) (Variables|Default|GetMaxTorque))))) _x) (/ (.Y (Math|Vector|BreakVector (* (LocalVariables|GetadjustedTorquePercent) (Math|Conversions|ToFloat(Integer) (Variables|Default|GetMaxTorque))))) _y) (/ (.Z (Math|Vector|BreakVector (* (LocalVariables|GetadjustedTorquePercent) (Math|Conversions|ToFloat(Integer) (Variables|Default|GetMaxTorque))))) _z))))

(fn GetAngularThrustPercenttoBrake
  (params (CurrentAngularVelocity :type Float%20%28single-precision%29) (MomentOfInertia :type Float%20%28single-precision%29))
  (bind _returnvalue (Utilities|Time|GetWorldDeltaSeconds))
  (bind _maxtorque (Variables|Default|GetMaxTorque))
  (bind _returnvalue_2 (/ CurrentAngularVelocity _returnvalue))
  (bind _returnvalue_3 (Math|Conversions|ToFloat(Integer) _maxtorque))
  (bind _returnvalue_4 (* MomentOfInertia _returnvalue_2))
  (if (!= CurrentAngularVelocity 0.0)
    (if (> (Math|Float|Absolute(Float) _returnvalue_4) _returnvalue_3)
      (if (> CurrentAngularVelocity 0.0)
        (LocalVariables|SetATP -1.0)
        (else
          (LocalVariables|SetATP 1.0)))
      (else
        (LocalVariables|SetATP (/ _returnvalue_4 _returnvalue_3))))
    (else
      (LocalVariables|SetATP 0.0)))
  (return (LocalVariables|GetATP)))

(fn GetStrafeThrusttoBreak
  (bind _returnvalue (Utilities|Time|GetWorldDeltaSeconds))
  (bind _returnvalue_2 (Utilities|Time|GetWorldDeltaSeconds))
  (bind _mass (Variables|Default|GetMass))
  (bind _maxstrafethrust (Variables|Default|GetMaxStrafeThrust))
  (bind _currentvelocity (Variables|Default|GetCurrentVelocity))
  (bind _currentvelocity_2 (Variables|Default|GetCurrentVelocity))
  (bind _mass_2 (Variables|Default|GetMass))
  (bind _maxstrafethrust_2 (Variables|Default|GetMaxStrafeThrust))
  (bind _returnvalue_3 (Math|Conversions|ToFloat(Integer) _maxstrafethrust_2))
  (bind _returnvalue_4 (Math|Conversions|ToFloat(Integer) _maxstrafethrust))
  (bind _z (Math|Vector|BreakVector _currentvelocity))
  (bind _y (Math|Vector|BreakVector _currentvelocity_2))
  (bind _returnvalue_5 (/ _y _returnvalue))
  (bind _returnvalue_6 (/ _z _returnvalue_2))
  (bind _returnvalue_7 (* _mass_2 _returnvalue_5))
  (bind _returnvalue_8 (* _mass _returnvalue_6))
  (if (!= _y 0.0)
    (if (> (Math|Float|Absolute(Float) _returnvalue_7) _returnvalue_3)
      (if (> (.Y (Math|Vector|BreakVector (Variables|Default|GetCurrentVelocity))) 0.0)
        (LocalVariables|SetthrustPercentY -1.0)
        (else
          (LocalVariables|SetthrustPercentY 1.0)))
      (else
        (LocalVariables|SetthrustPercentY (- 0.0 (/ _returnvalue_7 _returnvalue_3))))))
  (if (!= _z 0.0)
    (if (> (Math|Float|Absolute(Float) _returnvalue_8) _returnvalue_4)
      (if (> (.Z (Math|Vector|BreakVector (Variables|Default|GetCurrentVelocity))) 0.0)
        (LocalVariables|SetthrustPercentZ -1.0)
        (else
          (LocalVariables|SetthrustPercentZ 1.0)))
      (else
        (LocalVariables|SetthrustPercentZ (- 0.0 (/ _returnvalue_8 _returnvalue_4))))))
  (return (Math|Vector|MakeVector (.X (Math|Vector|BreakVector (Variables|Default|GetCurrentLinearThrustPercent))) (LocalVariables|GetthrustPercentY) (LocalVariables|GetthrustPercentZ))))