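; Player-controllable flying ship with six-axis movement driven by simple hand-written Newtonian physics.
; Input axes set thrust and torque percentages, which helper functions scale by maximum values and divide by mass or per-axis moment of inertia.
; Tick integrates these accelerations into persistent velocities without damping, then applies swept local offsets and unswept local rotations.
; Debug prints report linear velocity and angular acceleration.
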(event EventTick
  (params (DeltaSeconds :type Float%20%28single-precision%29))
  ;[1 1 1] Calculate linear and rotational accelerations, apply to velocities and update location and rotation
  (bind _linearacceleration (CallFunction|GetLinearAcceleration))
  (Development|PrintString (Utilities|String|BuildString(Vector) "" "Linear Velocity:" (+ (* _linearacceleration DeltaSeconds) (Variables|Default|GetCurrentVelocity))) false false)
  (Variables|Default|SetCurrentVelocity (+ (* _linearacceleration DeltaSeconds) (Variables|Default|GetCurrentVelocity)))
  (Transformation|AddActorLocalOffset (* (Variables|Default|GetCurrentVelocity) (Utilities|Time|GetWorldDeltaSeconds)) true)
  (bind _angularacceleration (CallFunction|GetAngularAcceleration))
  (Variables|Default|SetCurrentAngularVelocity (Math|Rotator|CombineRotators (* _angularacceleration (Utilities|Time|GetWorldDeltaSeconds)) (Variables|Default|GetCurrentAngularVelocity)))
  (Transformation|AddActorLocalRotation (* (Variables|Default|GetCurrentAngularVelocity) (Utilities|Time|GetWorldDeltaSeconds)) false))

(event Input|AxisEvents|InputAxisThrust
  (params (AxisValue :type Float%20%28single-precision%29))
  ;[1 1 1] Calculate X part of thrust percent
  (Variables|Default|SetCurrentLinearThrustPercent (Math|Vector|MakeVector AxisValue (.Y (Math|Vector|BreakVector (Variables|Default|GetCurrentLinearThrustPercent))) (.Z (Math|Vector|BreakVector (Variables|Default|GetCurrentLinearThrustPercent))))))

(event Input|AxisEvents|InputAxisStrafeHorizontal
  (params (AxisValue :type Float%20%28single-precision%29))
  ;[1 1 1] Calculate horizontal linear thrust (strafe)
  (Variables|Default|SetCurrentLinearThrustPercent (Math|Vector|MakeVector (.X (Math|Vector|BreakVector (Variables|Default|GetCurrentLinearThrustPercent))) AxisValue (.Z (Math|Vector|BreakVector (Variables|Default|GetCurrentLinearThrustPercent))))))

(event Input|AxisEvents|InputAxisStrafeVertical
  (params (AxisValue :type Float%20%28single-precision%29))
  ;[1 1 1] Calculate Vertical Linear Thrust (strafe)
  (Development|PrintString (Utilities|String|BuildString(Float) "" "Vertical Thrust Axis Value: " AxisValue) false false)
  (Variables|Default|SetCurrentLinearThrustPercent (Math|Vector|MakeVector (.X (Math|Vector|BreakVector (Variables|Default|GetCurrentLinearThrustPercent))) (.Y (Math|Vector|BreakVector (Variables|Default|GetCurrentLinearThrustPercent))) AxisValue)))

(event Input|AxisEvents|InputAxisPitch
  (params (AxisValue :type Float%20%28single-precision%29))
  ;[1 1 1] Calculate pitch Torque Percent
  (Variables|Default|SetCurrentTorquePercent (Math|Vector|MakeVector AxisValue (.Y (Math|Vector|BreakVector (Variables|Default|GetCurrentTorquePercent))) (.Z (Math|Vector|BreakVector (Variables|Default|GetCurrentTorquePercent))))))

(event Input|AxisEvents|InputAxisYaw
  (params (AxisValue :type Float%20%28single-precision%29))
  ;[1 1 1] Calculate Yaw Torque Percent
  (Variables|Default|SetCurrentTorquePercent (Math|Vector|MakeVector (.X (Math|Vector|BreakVector (Variables|Default|GetCurrentTorquePercent))) AxisValue (.Z (Math|Vector|BreakVector (Variables|Default|GetCurrentTorquePercent))))))

(event Input|AxisEvents|InputAxisRoll
  (params (AxisValue :type Float%20%28single-precision%29))
  ;[1 1 1] Calculate Yaw Roll Percent
  (Variables|Default|SetCurrentTorquePercent (Math|Vector|MakeVector (.X (Math|Vector|BreakVector (Variables|Default|GetCurrentTorquePercent))) (.Y (Math|Vector|BreakVector (Variables|Default|GetCurrentTorquePercent))) AxisValue)))

(fn ConstructionScript)

(fn GetLinearAcceleration
  (bind _currentlinearthrustpercent (Variables|Default|GetCurrentLinearThrustPercent))
  (bind _maxreversethrust (Variables|Default|GetMaxReverseThrust))
  (bind _maxforwardthrust (Variables|Default|GetMaxForwardThrust))
  (bind _maxstrafethrust (Variables|Default|GetMaxStrafeThrust))
  (bind (_x _y _z) (Math|Vector|BreakVector _currentlinearthrustpercent))
  (bind _returnvalue (* _maxstrafethrust _y))
  (bind _returnvalue_2 (* _maxstrafethrust _z))
  (if (< _x 0.0)
    (if (>= (Math|Float|Absolute(Float) _x) (Math|Conversions|ToFloat(Integer) (Variables|Default|GetMaxReverseThrust)))
      (LocalVariables|SetLinearThrust (Math|Vector|MakeVector (* -1 (Math|Conversions|ToFloat(Integer) _maxreversethrust)) _returnvalue _returnvalue_2))
      (else
        (LocalVariables|SetLinearThrust (Math|Vector|MakeVector (* _maxreversethrust _x) _returnvalue _returnvalue_2))))
    (elif (> _x (Math|Conversions|ToFloat(Integer) (Variables|Default|GetMaxForwardThrust)))
      (LocalVariables|SetLinearThrust (Math|Vector|MakeVector (Math|Conversions|ToFloat(Integer) _maxforwardthrust) _returnvalue _returnvalue_2))
      (else
        (LocalVariables|SetLinearThrust (Math|Vector|MakeVector (* (Math|Conversions|ToFloat(Integer) _maxforwardthrust) _x) _returnvalue _returnvalue_2)))))
  (return (/ (LocalVariables|GetLinearThrust) (Math|Conversions|ToFloat(Integer) (Variables|Default|GetMass)))))

(fn GetAngularAcceleration
  (bind _currenttorquepercent (Variables|Default|GetCurrentTorquePercent))
  (bind _maxtorque (Variables|Default|GetMaxTorque))
  (bind _momentofinertia (Variables|Default|GetMomentOfInertia))
  (bind _returnvalue (Math|Conversions|ToFloat(Integer) _maxtorque))
  (bind (_x _y _z) (Math|Vector|BreakVector _momentofinertia))
  (bind _returnvalue_2 (* _currenttorquepercent _returnvalue))
  (bind (_x_2 _y_2 _z_2) (Math|Vector|BreakVector _returnvalue_2))
  (bind _returnvalue_3 (/ _x_2 _x))
  (bind _returnvalue_4 (/ _y_2 _y))
  (bind _returnvalue_5 (/ _z_2 _z))
  (bind _returnvalue_6 (Class|KismetMathLibrary|MakeRot _returnvalue_3 _returnvalue_4 _returnvalue_5))
  (Development|PrintString (Class|KismetStringLibrary|BuildStringRotator "" "Angular Acceleration:" _returnvalue_6))
  (return _returnvalue_6))